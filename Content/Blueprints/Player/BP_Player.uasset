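; Player pawn for a burger-making game, holding ingredient stock, money and orders.
; Enhanced Input drives movement and facing, while a timeline lerps the camera to requested locations.
; Events process tomatoes and meat, deduct ingredients for completed burgers, and pay out when the made burger matches an order.
; B and M open the burger builder and meat grinder widgets with mouse cursor and UI focus.
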(event `self.ReceiveBeginPlay`
  (bind _asplayer_controller (cast `PlayerController` (`self.GetController`)))
  (bind _returnvalue (pcsubsystem `EnhancedInputLocalPlayerSubsystem` _asplayer_controller))
  (`/Engine/EditorBlueprintResources/StandardMacros.IsValid` _returnvalue
    (:`Is Valid`
      (`EnhancedInputSubsystemInterface.AddMappingContext` _returnvalue "/Game/Input/IMC_Default.IMC_Default" 0 (struct)))))

(event `EnhancedInput|/Game/Input/Actions/IA_Move`
  (params (ActionValue :type "Vector2D Structure") (ElapsedSeconds :type "Float (double-precision)") (TriggeredSeconds :type "Float (double-precision)") (InputAction :type "InputAction Object Reference" :default "/Game/Input/Actions/IA_Move.IA_Move"))
  (bind (_x _y) (`KismetMathLibrary.BreakVector2D` ActionValue))
  (bind _returnvalue (`KismetMathLibrary.Vector_Normal2D` (`KismetMathLibrary.MakeVector` _x _y)))
  (:`Triggered`
    (`self.K2_SetActorRotation` (`KismetMathLibrary.MakeRotFromX` _returnvalue))
    (`self.AddMovementInput` _returnvalue)))

(event `MoveCamera`
  (params (NewLoc :type "Vector Structure"))
  (set `self.OldCamLoc` (`SceneComponent.K2_GetComponentLocation` (`self.Camera`)))
  (set `self.NewCamLock` NewLoc)
  (bind (_direction _cammovetrack) (`Timeline|MoveCamTimeline` :!via `PlayFromStart`)
    (:`Update`
      (`SceneComponent.K2_SetWorldLocation` (`self.Camera`) (`KismetMathLibrary.VLerp` (`self.OldCamLoc`) (`self.NewCamLock`) _cammovetrack) false false))))

(event `Slice Tomatoes`
  (if (> (`self.Tomatoes`) 0)
    (set `self.Tomatoes` (- (`self.Tomatoes`) 1))
    (set `self.TomatoSlices` (+ (`self.TomatoSlices`) (`KismetMathLibrary.RandomIntegerInRange` 4 7)))))

(event `Grind Meat`
  (if (>= (`self.MeatPounds`) 25)
    (set `self.MeatPounds` (- (`self.MeatPounds`) 25))
    (`/Engine/EditorBlueprintResources/StandardMacros.IncrementInt` (`self.Patties`))))

(event `Check Orders`
  (bind _orders (`self.Orders`))
  (bind _made_burger (`self.Made Burger`))
  (bind (_made_burger_pattycount _made_burger_tomato _made_burger_lettuce) (break `/Game/Blueprints/ST_BurgerOrder` (`self.Made Burger`)))
  (if (`KismetArrayLibrary.Array_Contains` _orders _made_burger)
    (`KismetArrayLibrary.Array_Remove` _orders (`KismetArrayLibrary.Array_Find` _orders _made_burger))
    (set `self.TempCost` (* (`self.PattyCost`) _made_burger_pattycount))
    (if _made_burger_tomato
      (set `self.TempCost` (+ (`self.TempCost`) (`self.TomatoCost`))))
    (if _made_burger_lettuce
      (set `self.TempCost` (+ (`self.TempCost`) (`self.LettuceCost`))))
    (set `self.Money` (+ (`self.Money`) (`self.TempCost`)))
    (set `self.Made Burger` (make `/Game/Blueprints/ST_BurgerOrder` 0))
    (set `self.TempCost` 0)))

(event `Complete Burger`
  (params (Burger :type "/Game/Blueprints/ST_BurgerOrder Structure"))
  (set `self.CookedPatties` (- (`self.CookedPatties`) Burger_PattyCount_2_FCD9B20D4310FA638588009A811FCF90))
  (if Burger_Tomato_5_74070D204FD8B35F86AD7E8F3EBADC0B
    (`/Engine/EditorBlueprintResources/StandardMacros.DecrementInt` (`self.TomatoSlices`)
      (:`  `
        (if Burger_Lettuce_7_E714C15F488EFD18697B8EAE8F9C9899
          (`/Engine/EditorBlueprintResources/StandardMacros.DecrementInt` (`self.LettuceLeaves`)))))))

(event `Key|B`
  (params (Key :type "Key Structure"))
  (bind _returnvalue (`GameplayStatics.GetPlayerController` 0))
  (:`Pressed`
    (bind _returnvalue_2 (`|CreateWidget` "/Game/Blueprints/Widgets/W_BurgerBuilder.W_BurgerBuilder_C"))
    (`UserWidget.AddToViewport` _returnvalue_2 0)
    (set `PlayerController.bShowMouseCursor` true _returnvalue)
    (`WidgetBlueprintLibrary.SetInputMode_GameAndUIEx` _returnvalue _returnvalue_2)))

(event `Key|M`
  (params (Key :type "Key Structure"))
  (bind _returnvalue (`GameplayStatics.GetPlayerController` 0))
  (:`Pressed`
    (bind _returnvalue_2 (`|CreateWidget` "/Game/Blueprints/Widgets/W_MeatGrinder.W_MeatGrinder_C"))
    (`UserWidget.AddToViewport` _returnvalue_2 0)
    (set `PlayerController.bShowMouseCursor` true _returnvalue)
    (`WidgetBlueprintLibrary.SetInputMode_GameAndUIEx` _returnvalue _returnvalue_2)))

(fn `UserConstructionScript`)